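; Player controller for a rhythm game with four building lanes, two snare inputs and a bass input.
; On BeginPlay it finds the tagged buildings and starts a level sequence after a delay.
; Spawn functions queue notes per input, and each key press scores the oldest note by its height, destroys it and fires building Niagara effects.
; Lane and bass hits also shake the camera.
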(event `self.ReceiveBeginPlay`
  (set `self.Score` 0)
  (`|ExecutionSequence`
    (:`then_0`
      (bind _outactors (`GameplayStatics.GetAllActorsOfClass` "/Game/Desk/BP_Building.BP_Building_C"))
      (for _array_element _outactors
        (if (`self.ActorHasTag` _array_element "BuildA")
          (set `self.BuildA` _array_element)
          (elif (`self.ActorHasTag` _array_element "BuildZ")
            (set `self.BuildZ` _array_element)
            (elif (`self.ActorHasTag` _array_element "BuildE")
              (set `self.BuildE` _array_element)
              (elif (`self.ActorHasTag` _array_element "BuildR")
                (set `self.BuildR` _array_element)))))))
    (:`then_1`
      (`KismetSystemLibrary.Delay` 2.0)
      (bind _returnvalue (`GameplayStatics.GetActorOfClass` "/Script/LevelSequence.LevelSequenceActor"))
      (`MovieSceneSequencePlayer.Play` (`LevelSequenceActor.SequencePlayer` _returnvalue)))))

(event `InputAction|BuildAMapping`
  (params (Key :type "Key Structure"))
  (bind _buildanodes (`self.BuildANodes`))
  (bind _output (`|GetArrayItem` _buildanodes))
  (:`Pressed`
    (if (> (`KismetArrayLibrary.Array_Length` _buildanodes) 0)
      (`self.CheckForScoring` _output)
      (bind _asbp_building (cast `/Game/Desk/BP_Building` (`self.BuildA`)))
      (`/Game/Desk/BP_Building.ActiveNiagara` _asbp_building)
      (`self.K2_DestroyActor` _output)
      (`KismetArrayLibrary.Array_Remove` _buildanodes)
      (`GameplayStatics.PlayWorldCameraShake` "/Game/Camera/BP_Shake.BP_Shake_C" (`self.K2_GetActorLocation` (`self.BuildA`)) 0.0 5000.0))))

(event `InputAction|BuildZMapping`
  (params (Key :type "Key Structure"))
  (bind _buildznodes (`self.BuildZNodes`))
  (bind _output (`|GetArrayItem` _buildznodes))
  (:`Pressed`
    (if (> (`KismetArrayLibrary.Array_Length` _buildznodes) 0)
      (`self.CheckForScoring` _output)
      (bind _asbp_building (cast `/Game/Desk/BP_Building` (`self.BuildZ`)))
      (`/Game/Desk/BP_Building.ActiveNiagara` _asbp_building)
      (`self.K2_DestroyActor` _output)
      (`KismetArrayLibrary.Array_Remove` _buildznodes)
      (`GameplayStatics.PlayWorldCameraShake` "/Game/Camera/BP_Shake.BP_Shake_C" (`self.K2_GetActorLocation` (`self.BuildZ`)) 0.0 5000.0))))

(event `InputAction|BuildEMapping`
  (params (Key :type "Key Structure"))
  (bind _buildenodes (`self.BuildENodes`))
  (bind _output (`|GetArrayItem` _buildenodes))
  (:`Pressed`
    (if (> (`KismetArrayLibrary.Array_Length` _buildenodes) 0)
      (`self.CheckForScoring` _output)
      (bind _asbp_building (cast `/Game/Desk/BP_Building` (`self.BuildE`)))
      (`/Game/Desk/BP_Building.ActiveNiagara` _asbp_building)
      (`self.K2_DestroyActor` _output)
      (`KismetArrayLibrary.Array_Remove` _buildenodes)
      (`GameplayStatics.PlayWorldCameraShake` "/Game/Camera/BP_Shake.BP_Shake_C" (`self.K2_GetActorLocation` (`self.BuildE`)) 0.0 5000.0))))

(event `InputAction|BuildRMapping`
  (params (Key :type "Key Structure"))
  (bind _buildrnodes (`self.BuildRNodes`))
  (bind _output (`|GetArrayItem` _buildrnodes))
  (:`Pressed`
    (if (> (`KismetArrayLibrary.Array_Length` _buildrnodes) 0)
      (`self.CheckForScoring` _output)
      (bind _asbp_building (cast `/Game/Desk/BP_Building` (`self.BuildR`)))
      (`/Game/Desk/BP_Building.ActiveNiagara` _asbp_building)
      (`self.K2_DestroyActor` _output)
      (`KismetArrayLibrary.Array_Remove` _buildrnodes)
      (`GameplayStatics.PlayWorldCameraShake` "/Game/Camera/BP_Shake.BP_Shake_C" (`self.K2_GetActorLocation` (`self.BuildR`)) 0.0 5000.0))))

(event `InputAction|BuildLeftShiftMapping`
  (params (Key :type "Key Structure"))
  (bind _snarels (`self.SnareLS`))
  (bind _output (`|GetArrayItem` _snarels))
  (:`Pressed`
    (if (> (`KismetArrayLibrary.Array_Length` _snarels) 0)
      (`self.CheckForScoring` _output)
      (bind _asbp_building (cast `/Game/Desk/BP_Building` (`self.BuildA`)))
      (`/Game/Desk/BP_Building.ActiveNiagara` _asbp_building)
      (bind _asbp_building_2 (cast `/Game/Desk/BP_Building` (`self.BuildZ`)))
      (`/Game/Desk/BP_Building.ActiveNiagara` _asbp_building_2)
      (`self.K2_DestroyActor` _output)
      (`KismetArrayLibrary.Array_Remove` _snarels))))

(event `InputAction|BuildRightShiftMapping`
  (params (Key :type "Key Structure"))
  (bind _snarers (`self.SnareRS`))
  (bind _output (`|GetArrayItem` _snarers))
  (:`Pressed`
    (if (> (`KismetArrayLibrary.Array_Length` _snarers) 0)
      (`self.CheckForScoring` _output)
      (bind _asbp_building (cast `/Game/Desk/BP_Building` (`self.BuildE`)))
      (`/Game/Desk/BP_Building.ActiveNiagara` _asbp_building)
      (bind _asbp_building_2 (cast `/Game/Desk/BP_Building` (`self.BuildR`)))
      (`/Game/Desk/BP_Building.ActiveNiagara` _asbp_building_2)
      (`self.K2_DestroyActor` _output)
      (`KismetArrayLibrary.Array_Remove` _snarers))))

(event `InputAction|BuildSpaceMapping`
  (params (Key :type "Key Structure"))
  (bind _bass (`self.Bass`))
  (bind _output (`|GetArrayItem` _bass))
  (:`Pressed`
    (if (> (`KismetArrayLibrary.Array_Length` _bass) 0)
      (`self.CheckForScoring` _output)
      (bind _asbp_building (cast `/Game/Desk/BP_Building` (`self.BuildA`)))
      (`/Game/Desk/BP_Building.ActiveNiagara` _asbp_building)
      (bind _asbp_building_2 (cast `/Game/Desk/BP_Building` (`self.BuildZ`)))
      (`/Game/Desk/BP_Building.ActiveNiagara` _asbp_building_2)
      (bind _asbp_building_3 (cast `/Game/Desk/BP_Building` (`self.BuildE`)))
      (`/Game/Desk/BP_Building.ActiveNiagara` _asbp_building_3)
      (bind _asbp_building_4 (cast `/Game/Desk/BP_Building` (`self.BuildR`)))
      (`/Game/Desk/BP_Building.ActiveNiagara` _asbp_building_4)
      (`self.K2_DestroyActor` _output)
      (`KismetArrayLibrary.Array_Remove` _bass)
      (`GameplayStatics.PlayWorldCameraShake` "/Game/Camera/BP_ShakeBass.BP_ShakeBass_C" (`self.SpawnBassPoint`) 0.0 5000.0))))

(fn `CheckForScoring`
  (params (Node :type "Actor Object Reference"))
  (bind (_returnvalue_x _returnvalue_y _returnvalue_z) (`KismetMathLibrary.BreakVector` (`self.K2_GetActorLocation` Node)))
  (if (> _returnvalue_z (`self.ScorePoint`))
    (set `self.Score` (`KismetMathLibrary.FTrunc` (+ (/ (- 840.0 _returnvalue_z) 10.0) (`self.Score`))))
    (else
      (set `self.Score` (`KismetMathLibrary.FTrunc` (+ (`self.Score`) (/ _returnvalue_z 10.0)))))))

(fn `GetListOfActor`
  (params (Actor :type "Actor Object Reference"))
  (returns (List :type Integer))
  (for _array_element (`self.BuildANodes`)
    (if (== _array_element Actor)
      (return 0)
      (else
        (for _array_element_2 (`self.BuildZNodes`)
          (if (== _array_element_2 Actor)
            (return 1)
            (else
              (for _array_element_3 (`self.BuildENodes`)
                (if (== _array_element_3 Actor)
                  (return 2)
                  (else
                    (for _array_element_4 (`self.BuildRNodes`)
                      (if (== _array_element_4 Actor)
                        (return 3)))))))))))))

(fn `SpawnBass`
  (params (Pos :type "Vector Structure"))
  (bind _returnvalue (`|SpawnActorFromClass` "/Game/Desk/BP_NodeBasse.BP_NodeBasse_C" (`KismetMathLibrary.Conv_VectorToTransform` Pos) "Undefined" "MultiplyWithRoot" null null))
  (`KismetArrayLibrary.Array_Add` (`self.Bass`) _returnvalue))

(fn `SpawnLongNode`
  (params (Building :type "Actor Object Reference"))
  (bind _asbp_building (cast `/Game/Desk/BP_Building` Building))
  (bind _returnvalue (`KismetMathLibrary.Conv_VectorToTransform` (`self.K2_GetActorLocation` _asbp_building)))
  (bind _returnvalue_2 (`|SpawnActorFromClass` "/Game/Desk/BP_LongNode.BP_LongNode_C" (`KismetMathLibrary.Conv_VectorToTransform` (`KismetMathLibrary.MakeVector` (- (.x (.location _returnvalue)) 40.0) (.y (.location _returnvalue)) (.z (.location _returnvalue)))) "Undefined" "MultiplyWithRoot" null null))
  (if (== Building (`self.BuildA`))
    (`KismetArrayLibrary.Array_Add` (`self.BuildANodes`) _returnvalue_2)
    (elif (== Building (`self.BuildZ`))
      (`KismetArrayLibrary.Array_Add` (`self.BuildZNodes`) _returnvalue_2)
      (elif (== Building (`self.BuildE`))
        (`KismetArrayLibrary.Array_Add` (`self.BuildENodes`) _returnvalue_2)
        (elif (== Building (`self.BuildR`))
          (`KismetArrayLibrary.Array_Add` (`self.BuildRNodes`) _returnvalue_2))))))

(fn `SpawnNodeBasicA`
  (params (Building :type "Actor Object Reference"))
  (bind _returnvalue (`|SpawnActorFromClass` "/Game/Desk/BP_Node.BP_Node_C" (`KismetMathLibrary.Conv_VectorToTransform` (`self.SpawnPointA`)) "Undefined" "MultiplyWithRoot" null null))
  (if (== Building (`self.BuildA`))
    (`KismetArrayLibrary.Array_Add` (`self.BuildANodes`) _returnvalue)
    (elif (== Building (`self.BuildZ`))
      (`KismetArrayLibrary.Array_Add` (`self.BuildZNodes`) _returnvalue)
      (elif (== Building (`self.BuildE`))
        (`KismetArrayLibrary.Array_Add` (`self.BuildENodes`) _returnvalue)
        (elif (== Building (`self.BuildR`))
          (`KismetArrayLibrary.Array_Add` (`self.BuildRNodes`) _returnvalue))))))

(fn `SpawnNodeBasicE`
  (params (Building :type "Actor Object Reference"))
  (bind _returnvalue (`|SpawnActorFromClass` "/Game/Desk/BP_Node.BP_Node_C" (`KismetMathLibrary.Conv_VectorToTransform` (`self.SpawnPointE`)) "Undefined" "MultiplyWithRoot" null null))
  (if (== Building (`self.BuildA`))
    (`KismetArrayLibrary.Array_Add` (`self.BuildANodes`) _returnvalue)
    (elif (== Building (`self.BuildZ`))
      (`KismetArrayLibrary.Array_Add` (`self.BuildZNodes`) _returnvalue)
      (elif (== Building (`self.BuildE`))
        (`KismetArrayLibrary.Array_Add` (`self.BuildENodes`) _returnvalue)
        (elif (== Building (`self.BuildR`))
          (`KismetArrayLibrary.Array_Add` (`self.BuildRNodes`) _returnvalue))))))

(fn `SpawnNodeBasicR`
  (params (Building :type "Actor Object Reference"))
  (bind _returnvalue (`|SpawnActorFromClass` "/Game/Desk/BP_Node.BP_Node_C" (`KismetMathLibrary.Conv_VectorToTransform` (`self.SpawnPointR`)) "Undefined" "MultiplyWithRoot" null null))
  (if (== Building (`self.BuildA`))
    (`KismetArrayLibrary.Array_Add` (`self.BuildANodes`) _returnvalue)
    (elif (== Building (`self.BuildZ`))
      (`KismetArrayLibrary.Array_Add` (`self.BuildZNodes`) _returnvalue)
      (elif (== Building (`self.BuildE`))
        (`KismetArrayLibrary.Array_Add` (`self.BuildENodes`) _returnvalue)
        (elif (== Building (`self.BuildR`))
          (`KismetArrayLibrary.Array_Add` (`self.BuildRNodes`) _returnvalue))))))

(fn `SpawnNodeBasicZ`
  (params (Building :type "Actor Object Reference"))
  (bind _returnvalue (`|SpawnActorFromClass` "/Game/Desk/BP_Node.BP_Node_C" (`KismetMathLibrary.Conv_VectorToTransform` (`self.SpawnPointZ`)) "Undefined" "MultiplyWithRoot" null null))
  (if (== Building (`self.BuildA`))
    (`KismetArrayLibrary.Array_Add` (`self.BuildANodes`) _returnvalue)
    (elif (== Building (`self.BuildZ`))
      (`KismetArrayLibrary.Array_Add` (`self.BuildZNodes`) _returnvalue)
      (elif (== Building (`self.BuildE`))
        (`KismetArrayLibrary.Array_Add` (`self.BuildENodes`) _returnvalue)
        (elif (== Building (`self.BuildR`))
          (`KismetArrayLibrary.Array_Add` (`self.BuildRNodes`) _returnvalue))))))

(fn `SpawnSnare`
  (params (Pos :type "Vector Structure"))
  (bind (_spawnsnarelspoint_x _spawnsnarelspoint_y) (`KismetMathLibrary.BreakVector` (`self.SpawnSnareLSPoint`)))
  (bind _returnvalue (`|SpawnActorFromClass` "/Game/Desk/BP_NodeSnare.BP_NodeSnare_C" (`KismetMathLibrary.Conv_VectorToTransform` (`KismetMathLibrary.MakeVector` Pos_X Pos_Y Pos_Z)) "Undefined" "MultiplyWithRoot" null null))
  (if (== Pos_Y _spawnsnarelspoint_y)
    (`KismetArrayLibrary.Array_Add` (`self.SnareLS`) _returnvalue)
    (else
      (`KismetArrayLibrary.Array_Add` (`self.SnareRS`) _returnvalue))))

(fn `UserConstructionScript`)