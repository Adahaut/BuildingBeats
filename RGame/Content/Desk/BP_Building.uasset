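; BP_Building is a building actor that displays hit-rating feedback, apparently for a rhythm game, and changes its look on demand.
; Custom events flash Perfect, Nice, Good or Cross for a fraction of a second, hiding siblings, with a separate Bass set; ActiveBass duplicates ActiveCross.
; SETColor applies an indexed material to the spheres and cylinder and sets IsActive.
; REMM applies yellow hologram without clearing that flag, and ActiveNiagara triggers the particle system.
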(event `Active Perfect`
  (`SceneComponent.SetVisibility` (`self.Perfect`) true false)
  (`SceneComponent.SetVisibility` (`self.Good`) false false)
  (`SceneComponent.SetVisibility` (`self.Cross`) false false)
  (`SceneComponent.SetVisibility` (`self.Nice`) false false)
  (`KismetSystemLibrary.Delay` 0.2)
  (`SceneComponent.SetVisibility` (`self.Perfect`) false false))

(event `Active Nice`
  (`SceneComponent.SetVisibility` (`self.Nice`) true false)
  (`SceneComponent.SetVisibility` (`self.Good`) false false)
  (`SceneComponent.SetVisibility` (`self.Cross`) false false)
  (`SceneComponent.SetVisibility` (`self.Perfect`) false false)
  (`KismetSystemLibrary.Delay` 0.2)
  (`SceneComponent.SetVisibility` (`self.Nice`) false false))

(event `Active Good`
  (`SceneComponent.SetVisibility` (`self.Good`) true false)
  (`SceneComponent.SetVisibility` (`self.Cross`) false false)
  (`SceneComponent.SetVisibility` (`self.Nice`) false false)
  (`SceneComponent.SetVisibility` (`self.Perfect`) false false)
  (`KismetSystemLibrary.Delay` 0.2)
  (`SceneComponent.SetVisibility` (`self.Good`) false false))

(event `Active Cross`
  (`SceneComponent.SetVisibility` (`self.Cross`) true false)
  (`SceneComponent.SetVisibility` (`self.Good`) false false)
  (`SceneComponent.SetVisibility` (`self.Nice`) false false)
  (`SceneComponent.SetVisibility` (`self.Perfect`) false false)
  (`KismetSystemLibrary.Delay` 0.2)
  (`SceneComponent.SetVisibility` (`self.Cross`) false false))

(event `Active Bass`
  (`SceneComponent.SetVisibility` (`self.Cross`) true false)
  (`SceneComponent.SetVisibility` (`self.Good`) false false)
  (`SceneComponent.SetVisibility` (`self.Nice`) false false)
  (`SceneComponent.SetVisibility` (`self.Perfect`) false false)
  (`KismetSystemLibrary.Delay` 0.2)
  (`SceneComponent.SetVisibility` (`self.Cross`) false false))

(event `Active Perfect Bass`
  (`SceneComponent.SetVisibility` (`self.PerfectBass`) true false)
  (`SceneComponent.SetVisibility` (`self.GoodBass`) false false)
  (`SceneComponent.SetVisibility` (`self.CrossBass`) false false)
  (`SceneComponent.SetVisibility` (`self.NiceBass`) false false)
  (`KismetSystemLibrary.Delay` 0.2)
  (`SceneComponent.SetVisibility` (`self.PerfectBass`) false false))

(event `Active Nice Bass`
  (`SceneComponent.SetVisibility` (`self.NiceBass`) true false)
  (`SceneComponent.SetVisibility` (`self.GoodBass`) false false)
  (`SceneComponent.SetVisibility` (`self.CrossBass`) false false)
  (`SceneComponent.SetVisibility` (`self.PerfectBass`) false false)
  (`KismetSystemLibrary.Delay` 0.2)
  (`SceneComponent.SetVisibility` (`self.NiceBass`) false false))

(event `Active Good Bass`
  (`SceneComponent.SetVisibility` (`self.GoodBass`) true false)
  (`SceneComponent.SetVisibility` (`self.CrossBass`) false false)
  (`SceneComponent.SetVisibility` (`self.NiceBass`) false false)
  (`SceneComponent.SetVisibility` (`self.PerfectBass`) false false)
  (`KismetSystemLibrary.Delay` 0.2)
  (`SceneComponent.SetVisibility` (`self.GoodBass`) false false))

(event `Active Cross Bass`
  (`SceneComponent.SetVisibility` (`self.CrossBass`) true false)
  (`SceneComponent.SetVisibility` (`self.GoodBass`) false false)
  (`SceneComponent.SetVisibility` (`self.NiceBass`) false false)
  (`SceneComponent.SetVisibility` (`self.PerfectBass`) false false)
  (`KismetSystemLibrary.Delay` 0.2)
  (`SceneComponent.SetVisibility` (`self.CrossBass`) false false))

(fn `ActiveNiagara`
  (`ActorComponent.Activate` (`self.NewNiagaraSystem`) true))

(fn `REMM`
  (`PrimitiveComponent.SetMaterial` (`self.Sphere`) 0 "/Game/Material/M_HologramYellow.M_HologramYellow")
  (`PrimitiveComponent.SetMaterial` (`self.Cylinder`) 0 "/Game/Material/M_HologramYellow.M_HologramYellow")
  (`PrimitiveComponent.SetMaterial` (`self.Sphere1`) 0 "/Game/Material/M_HologramYellow.M_HologramYellow"))

(fn `SETColor`
  (params (MatNb :type Integer))
  (`PrimitiveComponent.SetMaterial` (`self.Sphere`) 0 (`|GetArrayItem` (`self.Materials`) MatNb))
  (`PrimitiveComponent.SetMaterial` (`self.Sphere1`) 0 (`|GetArrayItem` (`self.Materials`) MatNb))
  (`PrimitiveComponent.SetMaterial` (`self.Cylinder`) 0 (`|GetArrayItem` (`self.Materials`) MatNb))
  (set `self.IsActive` true))

(fn `UserConstructionScript`)