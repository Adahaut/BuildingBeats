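; BP_Destroyer is an actor that destroys any actor overlapping it and clears it from the player controller's tracking arrays.
; On overlap it destroys the other actor, then casts player 0's controller to BP_PlayerController.
; A nested chain tries removing the actor from the A, Z, E and R node arrays, then the bass and two snare arrays, stopping at the first successful removal.
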(event `self.ReceiveActorBeginOverlap`
  (params (OtherActor :type "Actor Object Reference"))
  (`self.K2_DestroyActor` OtherActor)
  (bind _asbp_player_controller (cast `/Game/Player/BP_PlayerController` (`GameplayStatics.GetPlayerController` 0)))
  (bind _returnvalue (`KismetArrayLibrary.Array_RemoveItem` (`/Game/Player/BP_PlayerController.BuildANodes` _asbp_player_controller) OtherActor))
  (if (not _returnvalue)
    (bind _returnvalue_2 (`KismetArrayLibrary.Array_RemoveItem` (`/Game/Player/BP_PlayerController.BuildZNodes` _asbp_player_controller) OtherActor))
    (if (not _returnvalue_2)
      (bind _returnvalue_3 (`KismetArrayLibrary.Array_RemoveItem` (`/Game/Player/BP_PlayerController.BuildENodes` _asbp_player_controller) OtherActor))
      (if (not _returnvalue_3)
        (bind _returnvalue_4 (`KismetArrayLibrary.Array_RemoveItem` (`/Game/Player/BP_PlayerController.BuildRNodes` _asbp_player_controller) OtherActor))
        (if (not _returnvalue_4)
          (bind _returnvalue_5 (`KismetArrayLibrary.Array_RemoveItem` (`/Game/Player/BP_PlayerController.Bass` _asbp_player_controller) OtherActor))
          (if (not _returnvalue_5)
            (bind _returnvalue_6 (`KismetArrayLibrary.Array_RemoveItem` (`/Game/Player/BP_PlayerController.SnareLS` _asbp_player_controller) OtherActor))
            (if (not _returnvalue_6)
              (`KismetArrayLibrary.Array_RemoveItem` (`/Game/Player/BP_PlayerController.SnareRS` _asbp_player_controller) OtherActor))))))))

(fn `UserConstructionScript`)